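; BP_Item is an interaction-system item actor that shows proximity icons to the player.
; Two sphere collisions react only to the player pawn: the outer shows or hides the distant icon, and the inner swaps it for the close-up icon.
; The construction script applies the configurable mesh and both sphere radii, so each instance can be tuned.
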(event OnComponentBeginOverlap(InnerSphereCollision)
  (params (OverlappedComponent :type Primitive%20Component%20Object%20Reference) (OtherActor :type Actor%20Object%20Reference) (OtherComp :type Primitive%20Component%20Object%20Reference) (OtherBodyIndex :type Integer) (bFromSweep :type Boolean) (SweepResult :type Hit%20Result%20Structure%20%28by%20ref%29))
  (if (== OtherActor (Game|Player|GetPlayerPawn 0))
    (Rendering|SetVisibility (Variables|Default|GetCloseUpIcon) true false)
    (Rendering|SetVisibility (Variables|Default|GetDistantIcon) false false)))

(event OnComponentEndOverlap(InnerSphereCollision)
  (params (OverlappedComponent :type Primitive%20Component%20Object%20Reference) (OtherActor :type Actor%20Object%20Reference) (OtherComp :type Primitive%20Component%20Object%20Reference) (OtherBodyIndex :type Integer))
  (if (== (Game|Player|GetPlayerPawn 0) OtherActor)
    (Rendering|SetVisibility (Variables|Default|GetCloseUpIcon) false false)
    (Rendering|SetVisibility (Variables|Default|GetDistantIcon) true false)))

(event OnComponentBeginOverlap(OuterSphereCollision)
  (params (OverlappedComponent :type Primitive%20Component%20Object%20Reference) (OtherActor :type Actor%20Object%20Reference) (OtherComp :type Primitive%20Component%20Object%20Reference) (OtherBodyIndex :type Integer) (bFromSweep :type Boolean) (SweepResult :type Hit%20Result%20Structure%20%28by%20ref%29))
  (if (== OtherActor (Game|Player|GetPlayerPawn 0))
    (Rendering|SetVisibility (Variables|Default|GetDistantIcon) true false)))

(event OnComponentEndOverlap(OuterSphereCollision)
  (params (OverlappedComponent :type Primitive%20Component%20Object%20Reference) (OtherActor :type Actor%20Object%20Reference) (OtherComp :type Primitive%20Component%20Object%20Reference) (OtherBodyIndex :type Integer))
  (if (== (Game|Player|GetPlayerPawn 0) OtherActor)
    (Rendering|SetVisibility (Variables|Default|GetDistantIcon) false false)))

(fn ConstructionScript
  (Components|Sphere|SetSphereRadius (Variables|Default|GetInnerSphereCollision) (Variables|ItemSettings|GetInnerSphereRadius) true)
  (Components|Sphere|SetSphereRadius (Variables|Default|GetOuterSphereCollision) (Variables|ItemSettings|GetOuterSphereRadius) true)
  (Components|StaticMesh|SetStaticMesh (Variables|Default|GetStaticMesh) (Variables|ItemSettings|GetItemMesh)))