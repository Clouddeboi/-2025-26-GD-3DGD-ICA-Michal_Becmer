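; BP_PuzzleBox is an interactable puzzle box item that plays an animation the first time it is interacted with.
; The construction script applies the configured skeletal mesh and world scale to the component.
; On Interact, it reapplies the mesh, switches to single-node animation mode and plays the chosen animation once without looping.
; A boolean flag then blocks any further interaction.
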(event EventBeginPlay
  (|CallParentFunction) ; This node is disabled and will not be called.\nDrag off pins to build functionality.
)

(event EventInteract
  (params (Interacter :type BP%20First%20Person%20Character%20Object%20Reference))
  (if (not (Variables|Default|GetAlreadyInteractedWithBox))
    (Components|SkeletalMesh|SetSkeletalMeshAsset (Variables|Default|GetSkeletalMesh) (Variables|Default|GetObjectSkeletalMesh))
    (Components|Animation|SetAnimationMode (Variables|Default|GetSkeletalMesh) "AnimationSingleNode" true)
    (Components|Animation|PlayAnimation (Variables|Default|GetSkeletalMesh) (Variables|Default|GetAnimationToPlay) false)
    (Variables|Default|SetAlreadyInteractedWithBox true)))

(fn ConstructionScript
  (bind _skeletalmesh (Variables|Default|GetSkeletalMesh))
  (|CallParentFunction)
  (Components|SkeletalMesh|SetSkeletalMeshAsset _skeletalmesh (Variables|Default|GetObjectSkeletalMesh))
  (Transformation|SetWorldScale3D _skeletalmesh (Variables|Default|GetObjectScale)))