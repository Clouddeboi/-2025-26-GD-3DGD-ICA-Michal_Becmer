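; BP_LightSwitch is an interactable light switch item that turns groups of spot and point lights off and on.
; Each Interact call alternates a FlipFlop that sets LightsOff and loops over the SpotLights and PointLights arrays, zeroing intensity or restoring hardcoded low values per light type.
; The first interaction always switches the lights off.
; The construction script runs the parent's, then positions the static mesh at ObjectMeshLocation.
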(event EventInteract
  (params (Interacter :type BP%20First%20Person%20Character%20Object%20Reference))
  (Utilities|FlowControl|FlipFlop
    (:A
      (Variables|Default|SetLightsOff? true)
      (for _array_element (Variables|Default|GetSpotLights)
        (Rendering|Components|Light|SetIntensity (Variables|/Script/Engine.SpotLight|GetSpotLightComponent _array_element) 0.0))
      (for _array_element_2 (Variables|Default|GetPointLights)
        (Rendering|Components|Light|SetIntensity (Variables|/Script/Engine.PointLight|GetPointLightComponent _array_element_2) 0.0)))
    (:B
      (Variables|Default|SetLightsOff? false)
      (for _array_element_3 (Variables|Default|GetSpotLights)
        (Rendering|Components|Light|SetIntensity (Variables|/Script/Engine.SpotLight|GetSpotLightComponent _array_element_3) 0.05))
      (for _array_element_4 (Variables|Default|GetPointLights)
        (Rendering|Components|Light|SetIntensity (Variables|/Script/Engine.PointLight|GetPointLightComponent _array_element_4) 0.14)))))

(fn ConstructionScript
  (|CallParentFunction)
  (Transformation|SetRelativeLocation (Variables|Default|GetStaticMesh) (Variables|Default|GetObjectMeshLocation) false false))