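; Chandelier actor in the item frame puzzle folder that descends 200 units when its LowerChandelier event is called.
; The construction script places the root at the stored WorldLocation variable, which also serves as the descent's start point.
; A timeline lerps the root from there to the lowered position without sweeping.
; GetLocation returns the stored WorldLocation, which stays unchanged as the chandelier moves.
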(event Custom|LowerChandelier
  (Variables|Default|SetStartLocation (Variables|Default|GetWorldLocation))
  (Variables|Default|SetEndLocation (- (Variables|Default|GetStartLocation) "0.000000,0.000000,200.000000"))
  (bind _alpha (Timeline|LowerChandelierTimeline Play)
    (:Update
      (Transformation|SetWorldLocation (Variables|Default|GetDefaultSceneRoot) (Math|Vector|Lerp(Vector) (Variables|Default|GetStartLocation) (Variables|Default|GetEndLocation) _alpha) false false))))

(fn ConstructionScript
  (Transformation|SetWorldLocation (Variables|Default|GetDefaultSceneRoot) (Variables|Default|GetWorldLocation) false false))

(fn GetLocation
  (return (Variables|Default|GetWorldLocation)))