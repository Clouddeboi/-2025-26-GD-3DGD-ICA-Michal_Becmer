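; BP_ItemFrame is an interactable puzzle frame that accepts a required item from the player's inventory to lower a chandelier.
; On Interact it searches the first-person character's inventory, then spawns a BP_TonyCereal at the attach point and plays placement and chain sounds.
; A one-time flag blocks repeat placement once it succeeds.
; The construction script positions the attach point from a configurable relative offset.
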(event EventBeginPlay
  (|CallParentFunction)
  (bind _returnvalue (Actor|GetActorOfClass "/Game/my_assets/Blueprints/Player/BP_FirstPersonCharacter.BP_FirstPersonCharacter_C"))
  (Variables|Default|SetPlayerReference _returnvalue)
  (bind _returnvalue_2 (Actor|GetActorOfClass "/Game/my_assets/Blueprints/Puzzle/ItemFramePuzzle/BP_Chandlier.BP_Chandlier_C"))
  (Variables|Default|SetChandlierReference _returnvalue_2))

(event EventInteract
  (params (Interacter :type BP%20First%20Person%20Character%20Object%20Reference))
  (bind _attachlocation (Variables|Default|GetAttachLocation))
  (bind _chandlierreference (Variables|Default|GetChandlierReference))
  (bind _returnvalue (Transformation|GetWorldLocation _attachlocation))
  (if (not (Variables|Default|GetAlreadyPlacedItem))
    (bind _doesplayerhaveitem_ (Default|SearchItems (Variables|/Game/my_assets/Blueprints/Player/BP_FirstPersonCharacter.BP_FirstPersonCharacter_C|GetInventoryReference (Variables|Default|GetPlayerReference)) (Variables|Default|GetItemRequiredForPuzzle)))
    (if _doesplayerhaveitem_
      (Variables|Default|SetHasItem true)
      (Game|SpawnActorfromClass "/Game/my_assets/Blueprints/Puzzle/ItemFramePuzzle/BP_TonyCereal.BP_TonyCereal_C" (Math|Transform|MakeTransform _returnvalue "0, 0, 0" "1.000000,1.000000,1.000000") "Undefined" "MultiplyWithRoot" 0 0)
      (Audio|PlaySoundatLocation "/Game/my_assets/Audio/Puzzle/Place.Place" _returnvalue "0, 0, 0" 1.0 1.0 0.0 0 0 0 0)
      (Default|LowerChandelier _chandlierreference)
      (bind _worldlocationforsound (Default|GetLocation _chandlierreference))
      (Audio|PlaySoundatLocation "/Game/my_assets/Audio/Puzzle/Chain.Chain" _worldlocationforsound "0, 0, 0" 1.0 1.0 0.0 0 0 0 0)
      (Variables|Default|SetAlreadyPlacedItem true)
      (else
        (Variables|Default|SetHasItem false)))))

(fn ConstructionScript
  (|CallParentFunction)
  (Transformation|SetRelativeLocation (Variables|Default|GetAttachLocation) (Variables|Default|GetObjectAttachLocation) false false))