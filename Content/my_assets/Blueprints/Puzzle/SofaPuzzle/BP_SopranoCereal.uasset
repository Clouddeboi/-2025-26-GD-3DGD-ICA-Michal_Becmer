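; BP_SopranoCereal is a sofa puzzle prop that supplies a text notification.
; Its construction script calls the parent's, then applies variable-driven world rotation and relative location to the static mesh.
; SendOutTextNotify returns the TextToDisplay0 variable regardless of the component passed in.
; The event graph has no active logic.
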(event EventBeginPlay
  (|CallParentFunction) ; This node is disabled and will not be called.\nDrag off pins to build functionality.
)

(fn ConstructionScript
  (bind _staticmesh (Variables|Default|GetStaticMesh))
  (|CallParentFunction)
  (Transformation|SetWorldRotation _staticmesh (Variables|Default|GetSetMeshRotation) false false)
  (Transformation|SetRelativeLocation _staticmesh (Variables|Default|GetSetMeshLocation) false false))

(fn SendOutTextNotify
  (params (Component :type Primitive%20Component%20Object%20Reference))
  (return (Variables|Default|GetText%20to%20Display_0)))