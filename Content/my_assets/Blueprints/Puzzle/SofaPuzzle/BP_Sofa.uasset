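; BP_Sofa is a sofa in the sofa puzzle that slides aside when interacted with.
; On Interact, it stores its current location, sets a target a fixed distance along world +X, and plays a moving sound at its position.
; The MoveSofa timeline then drives a lerp between the two points, moving the root component without sweep, so collisions do not block the slide.
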(event EventBeginPlay
  (|CallParentFunction) ; This node is disabled and will not be called.\nDrag off pins to build functionality.
)

(event EventInteract
  (params (Interacter :type BP%20First%20Person%20Character%20Object%20Reference))
  (Variables|Default|SetStartLocation (Transformation|GetWorldLocation (Variables|Default|GetDefaultSceneRoot)))
  (Variables|Default|SetEndLocation (+ (Variables|Default|GetStartLocation) "160.000000,0.000000,0.000000"))
  (Audio|PlaySoundatLocation "/Game/my_assets/Audio/Puzzle/SofaMove.SofaMove" (Transformation|GetWorldLocation (Variables|Default|GetDefaultSceneRoot)) "0, 0, 0" 1.0 1.0 0.0 0 0 0 0)
  (bind _alpha (Timeline|MoveSofa Play)
    (:Update
      (Transformation|SetWorldLocation (Variables|Default|GetDefaultSceneRoot) (Math|Vector|Lerp(Vector) (Variables|Default|GetStartLocation) (Variables|Default|GetEndLocation) _alpha) false false))))

(fn ConstructionScript
  (|CallParentFunction))