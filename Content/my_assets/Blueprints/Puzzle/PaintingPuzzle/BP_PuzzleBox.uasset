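; BP_PuzzleBox is an interactable puzzle box that opens or animates once when the player holds a required inventory item.
; The construction script applies a configurable skeletal mesh and scale, and BeginPlay caches the first-person character.
; Interact searches that character's inventory for the item, then plays a configurable single-node animation without looping, disables mesh collision and sets a flag blocking further use.
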(event EventBeginPlay
  (|CallParentFunction)
  (bind _returnvalue (Actor|GetActorOfClass "/Game/my_assets/Blueprints/Player/BP_FirstPersonCharacter.BP_FirstPersonCharacter_C"))
  (Variables|Default|SetPlayerReference _returnvalue))

(event EventInteract
  (params (Interacter :type BP%20First%20Person%20Character%20Object%20Reference))
  (if (not (Variables|Default|GetAlreadyInteractedWithBox))
    (bind _doesplayerhaveitem_ (Default|SearchItems (Variables|/Game/my_assets/Blueprints/Player/BP_FirstPersonCharacter.BP_FirstPersonCharacter_C|GetInventoryReference (Variables|Default|GetPlayerReference)) (Variables|Default|GetRequiredItem)))
    (if _doesplayerhaveitem_
      (Components|SkeletalMesh|SetSkeletalMeshAsset (Variables|Default|GetSkeletalMesh) (Variables|Default|GetObjectSkeletalMesh))
      (Components|Animation|SetAnimationMode (Variables|Default|GetSkeletalMesh) "AnimationSingleNode" true)
      (Components|Animation|PlayAnimation (Variables|Default|GetSkeletalMesh) (Variables|Default|GetAnimationToPlay) false)
      (Collision|SetCollisionEnabled (Variables|Default|GetSkeletalMesh) "NoCollision")
      (Variables|Default|SetAlreadyInteractedWithBox true))))

(fn ConstructionScript
  (bind _skeletalmesh (Variables|Default|GetSkeletalMesh))
  (|CallParentFunction)
  (Components|SkeletalMesh|SetSkeletalMeshAsset _skeletalmesh (Variables|Default|GetObjectSkeletalMesh))
  (Transformation|SetWorldScale3D _skeletalmesh (Variables|Default|GetObjectScale)))