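; BP_Door is a door Blueprint that swings open when its OpenDoor event is called.
; The event sets the Scene component's relative rotation to StartRotation, then plays OpenDoorTimeline, whose Alpha drives a rotator lerp toward EndRotation on each update.
; It has no closing logic, and the construction script is empty.
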(event Custom|OpenDoor
  (Transformation|SetRelativeRotation (Variables|Default|GetScene) (Variables|Default|GetStartRotation) false false)
  (Variables|Default|SetEndRotation (Variables|Default|GetEndRotation))
  (bind _alpha (Timeline|OpenDoorTimeline Play)
    (:Update
      (Transformation|SetRelativeRotation (Variables|Default|GetScene) (Math|Rotator|Lerp(Rotator) (Variables|Default|GetStartRotation) (Variables|Default|GetEndRotation) _alpha) false false))))

(fn ConstructionScript)