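; AC_Inventory is an inventory component that stores items in an Inventory array and provides search, add and remove functions.
; AddItem appends without any duplicate check, while SearchItems and RemoveItem loop through the array comparing item IDs.
; SearchItems sets an IsItemInInventory flag and returns it on a match, and RemoveItem deletes only the first matching entry by index.
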(fn SearchItems
  (params (Item :type S%20Item%20Data%20Structure))
  (for _array_element (Variables|Default|GetInventory)
    (if (== (.id _array_element) (.id Item))
      (Variables|Default|SetIsItemInInventory? true)
      (return (Variables|Default|GetIsItemInInventory?))
      (else
        (Variables|Default|SetIsItemInInventory? false)))))

(fn AddItem
  (params (Item :type S%20Item%20Data%20Structure))
  (Utilities|Array|Add (Variables|Default|GetInventory) Item))

(fn RemoveItem
  (params (Item :type S%20Item%20Data%20Structure))
  (bind (_array_element _array_index) (Utilities|Array|ForEachLoopwithBreak (Variables|Default|GetInventory) :!label _label)
    (:LoopBody
      (if (== (.id _array_element) (.id Item))
        (Utilities|Array|RemoveIndex (Variables|Default|GetInventory) _array_index)
        (goto _label Break)))))